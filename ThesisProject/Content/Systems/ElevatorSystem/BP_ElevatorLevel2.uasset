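; BP_ElevatorLevel2 is an elevator actor that opens its door automatically shortly after play begins.
; BeginPlay runs once through a DoOnce, waits briefly, plays the door sound in 2D, and starts a timeline that drives the door's relative Z position.
; When the timeline finishes, it hides the light and stops both audio components.
; The box overlap event is empty, so no trigger logic is involved.
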(event OnComponentBeginOverlap(Box)
  (params (OverlappedComponent :type Primitive%20Component%20Object%20Reference) (OtherActor :type Actor%20Object%20Reference) (OtherComp :type Primitive%20Component%20Object%20Reference) (OtherBodyIndex :type Integer) (bFromSweep :type Boolean) (SweepResult :type Hit%20Result%20Structure%20%28by%20ref%29)))

(event EventBeginPlay
  (bind _elevatordoor (Variables|Default|GetElevatorDoor))
  (bind _relativelocation (Variables|/Script/Engine.SceneComponent|GetRelativeLocation _elevatordoor))
  (Utilities|FlowControl|DoOnce false
    (:Completed
      (Utilities|FlowControl|Delay 3.0)
      (Audio|PlaySound2D "/Game/SFX/SoundEffects/General/ElevatorDoor.ElevatorDoor" 1.0 1.0 0.0 0 0)
      (bind _dooropen (Timeline|ElevatorDoorAnimation Play)
        (:Update
          (Transformation|SetRelativeLocation _elevatordoor (Math|Vector|MakeVector (.x _relativelocation) (.y _relativelocation) _dooropen) false false))
        (:Finished
          (Rendering|SetVisibility (Variables|Default|GetLight) false false)
          (Audio|Components|Audio|Stop (Variables|Default|GetAudio))
          (Audio|Components|Audio|Stop (Variables|Default|GetAudioLight)))))))

(event Collision|EventActorBeginOverlap
  (params (OtherActor :type Actor%20Object%20Reference)))

(event EventTick
  (params (DeltaSeconds :type Float%20%28single-precision%29)))

(fn ConstructionScript)