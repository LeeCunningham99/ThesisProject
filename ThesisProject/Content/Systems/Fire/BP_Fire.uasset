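; BP_Fire is a fire hazard that repeatedly hurts the player character while it overlaps the Collision component.
; BeginPlay caches the third-person character and starts a looping timer, while overlap begin and end events toggle a Burning flag.
; When burning, each timer tick feeds a Delay that throttles damage, then plays a 2D hurt sound and calls DamageTaken on the character.
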(event OnComponentBeginOverlap(Collision)
  (params (OverlappedComponent :type Primitive%20Component%20Object%20Reference) (OtherActor :type Actor%20Object%20Reference) (OtherComp :type Primitive%20Component%20Object%20Reference) (OtherBodyIndex :type Integer) (bFromSweep :type Boolean) (SweepResult :type Hit%20Result%20Structure%20%28by%20ref%29))
  (if (== OtherActor (Variables|Default|GetAs%20BP%20Third%20Person%20Character))
    (Variables|Default|SetBurning true)))

(event OnComponentEndOverlap(Collision)
  (params (OverlappedComponent :type Primitive%20Component%20Object%20Reference) (OtherActor :type Actor%20Object%20Reference) (OtherComp :type Primitive%20Component%20Object%20Reference) (OtherBodyIndex :type Integer))
  (if (== OtherActor (Variables|Default|GetAs%20BP%20Third%20Person%20Character))
    (Variables|Default|SetBurning false)))

(event Custom|IsBurning
  (if (Variables|Default|GetBurning)
    (Utilities|FlowControl|Delay 0.5)
    (Audio|PlaySound2D "/Game/SFX/SoundEffects/Player/PlayerHurt.PlayerHurt" 1.0 1.0 0.0 0 0)
    (Default|DamageTaken (Variables|Default|GetAs%20BP%20Third%20Person%20Character))))

(event EventBeginPlay
  (bind _asbp_third_person_character (Utilities|Casting|CastToBP_ThirdPersonCharacter (Game|GetPlayerCharacter 0)))
  (Variables|Default|SetAs%20BP%20Third%20Person%20Character _asbp_third_person_character)
  (Utilities|Time|SetTimerbyEvent (delegate Custom|IsBurning) 0.2 true))

(event EventTick
  (params (DeltaSeconds :type Float%20%28single-precision%29)))

(fn ConstructionScript)