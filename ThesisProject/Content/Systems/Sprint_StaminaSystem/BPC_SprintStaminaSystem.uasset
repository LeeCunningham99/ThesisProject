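; Sprint stamina component that switches walk and sprint speeds from IA_Sprint and creates the W_Stamina widget, toggling its visibility after delays.
; A looping timer drains stamina during grounded movement near sprint speed, otherwise regenerates it, broadcasting the percentage.
; Depletion forces walking, plays a one-shot sound and blocks sprinting until stamina is full.
; "Full" is a hardcoded threshold independent of MaxStamina, at which the timer can clear.
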(event Custom|SetupStaminaComponentReferences
  (params (Actor :type Actor%20Object%20Reference) (CharacterMovementComponent :type Character%20Movement%20Component%20Object%20Reference) (MovementSpeed :type F%20Speed%20Structure) (MaxStamina :type Float%20%28double-precision%29) (ExhaustedSound :type Sound%20Base%20Object%20Reference) (SprintingSound :type Sound%20Base%20Object%20Reference))
  ;[1 1 1] Stamina System Component References - SET
  (Variables|Default|SetActor Actor)
  (bind _output_get (Variables|Default|SetCharacter%20Movement%20Component CharacterMovementComponent))
  (bind _output_get_2 (Variables|Default|SetMovement%20Speed MovementSpeed))
  (Variables|/Script/Engine.CharacterMovementComponent|SetMaxWalkSpeed _output_get (.walking _output_get_2))
  (Variables|Default|SetMax%20Stamina MaxStamina)
  (Variables|Default|SetCurrentStamina MaxStamina)
  (Variables|Default|SetExhausted%20Sound ExhaustedSound)
  (Variables|Default|SetSprinting%20Sound SprintingSound)
  (bind _returnvalue (UserInterface|CreateWidget "/Game/Systems/Sprint_StaminaSystem/W_Stamina.W_Stamina_C" (Game|GetPlayerController 0)))
  (bind _output_get_3 (Variables|Default|SetStaminaUI _returnvalue))
  (UserInterface|Viewport|AddtoViewport _output_get_3 0))

(event Custom|StartStaminaCycle
  ;[1 1 1] Stamina Manager
  (bind _returnvalue (Utilities|Time|SetTimerbyEvent (delegate Custom|StartStaminaCycleManager) 0.5 true))
  (Variables|Default|SetStaminaTimerHandle _returnvalue))

(event Custom|StoppedSprinting
  ;[1 1 1] Clear Timer Once Stamina Is Full
  (if (CallFunction|GetStaminaFull)
    (Utilities|Time|ClearandInvalidateTimerbyHandle (Variables|Default|GetStaminaTimerHandle))))

(event Custom|EventOnExhausted
  ;[1 1 1] Exhaustion & Stamina Recovered
  (Utilities|FlowControl|Sequence
    (:then_0
      (CallFunction|StopSprinting))
    (:then_1
      (Utilities|FlowControl|DoOnce false
        (:Completed
          (Audio|PlaySound2D (Variables|Default|GetExhausted%20Sound) 1.0 1.0 0.0 0 0))))))

(event Custom|EventStaminaRecovered
  ;[1 1 1] Exhaustion & Stamina Recovered
  (Utilities|FlowControl|DoOnce false) ; enters at Reset
)

(event Custom|StartStaminaCycleManager
  ;[1 1 1] Stamina Manager
  (CallFunction|StaminaCycleManager (Variables|Default|GetCharacter%20Movement%20Component) (.sprinting (Variables|Default|GetMovement%20Speed))))

(event Input|EnhancedActionEvents|EnhancedInputActionIA_Sprint
  (params (ActionValue :type Boolean) (ElapsedSeconds :type Float%20%28double-precision%29) (TriggeredSeconds :type Float%20%28double-precision%29) (InputAction :type Input%20Action%20Object%20Reference :default "/Game/ThirdPerson/Input/Actions/IA_Sprint.IA_Sprint"))
  (bind _staminaui (Variables|Default|GetStaminaUI))
  ;[1 1 1] Sprinting Input Action & UI
  (:Started
    (CallFunction|StartSprinting)
    (Utilities|FlowControl|Delay 1.0)
    (Variables|/Script/UMG.Widget|SetVisibility _staminaui "Visible"))
  (:Completed
    (CallFunction|StopSprinting)
    (Utilities|FlowControl|Delay 1e+01)
    (Variables|/Script/UMG.Widget|SetVisibility _staminaui "Hidden")))

(fn StartSprinting
  (if (not (Variables|Default|GetIsExhausted?))
    (Variables|/Script/Engine.CharacterMovementComponent|SetMaxWalkSpeed (Variables|Default|GetCharacter%20Movement%20Component) (.sprinting (Variables|Default|GetMovement%20Speed)))
    (Variables|Default|SetSprintActionActive true)
    (CallFunction|StartStaminaCycle)))

(fn StopSprinting
  (Variables|/Script/Engine.CharacterMovementComponent|SetMaxWalkSpeed (Variables|Default|GetCharacter%20Movement%20Component) (.walking (Variables|Default|GetMovement%20Speed)))
  (Variables|Default|SetSprintActionActive false)
  (CallFunction|StoppedSprinting))

(fn StaminaCycleManager
  (params (CharacterMovementComponent :type Character%20Movement%20Component%20Object%20Reference) (SprintSpeedReference :type Float%20%28double-precision%29))
  (Utilities|StaminaDrainorRegen CharacterMovementComponent SprintSpeedReference
    (:StaminaDrain
      (CallFunction|DrainStamina)
      (if (not (CallFunction|GetStaminaFull))
        (Variables|Default|SetDrainCycleStarted true)
        (if (CallFunction|GetStaminaDepleted)
          (Variables|Default|SetIsExhausted? true)
          (CallFunction|EventonExhausted)
          (Default|CallCallonExhausted))))
    (:StaminaRegen
      (CallFunction|RegenStamina)
      (if (and (CallFunction|GetStaminaFull) (not (CallFunction|GetCurrentlySprinting CharacterMovementComponent SprintSpeedReference)))
        (Variables|Default|SetIsExhausted? false)
        (CallFunction|EventStaminaRecovered)
        (Default|CallCallStaminaRecovered)
        (if (Variables|Default|GetDrainCycleStarted)
          (if (CallFunction|GetStaminaFull)
            (Utilities|Time|ClearandInvalidateTimerbyHandle (Variables|Default|GetStaminaTimerHandle))
            (Variables|Default|SetDrainCycleStarted false)))))))

(fn GetCurrentlySprinting
  (params (CharacterMovementComponent :type Character%20Movement%20Component%20Object%20Reference) (SprintSpeedReference :type Float%20%28double-precision%29))
  (return (> (Math|Vector|VectorLength (Pawn|Components|CharacterMovement|GetLastUpdateVelocity CharacterMovementComponent)) (- SprintSpeedReference 3.0))))

(fn GetStaminaFull
  (return (>= (Variables|Default|GetCurrentStamina) 3e+01)))

(fn GetIsonGround
  (params (CharacterMovementComponent :type Character%20Movement%20Component%20Object%20Reference))
  (return (== (.z (Math|Vector|Normalize (Pawn|Components|CharacterMovement|GetLastUpdateVelocity CharacterMovementComponent))) 0.0)))

(fn DrainStamina
  (bind _output_get (Variables|Default|SetCurrentStamina (Math|Float|Clamp(Float) (- (Variables|Default|GetCurrentStamina) (Variables|Default|GetDrainAmount)) 0.0 (Variables|Default|GetMax%20Stamina))))
  (Default|CallCallUpdateStamina (CallFunction|GetStaminaPercentage _output_get))
  (return))

(fn GetStaminaPercentage
  (params (RawStamina :type Float%20%28double-precision%29))
  (return (/ RawStamina (Variables|Default|GetMax%20Stamina))))

(fn GetStaminaDepleted
  (return (<= (Variables|Default|GetCurrentStamina) 0.0)))

(fn RegenStamina
  (bind _output_get (Variables|Default|SetCurrentStamina (Math|Float|Clamp(Float) (+ (Variables|Default|GetCurrentStamina) (Variables|Default|GetRegenAmount)) 0.0 (Variables|Default|GetMax%20Stamina))))
  (Default|CallCallUpdateStamina (CallFunction|GetStaminaPercentage _output_get))
  (return))