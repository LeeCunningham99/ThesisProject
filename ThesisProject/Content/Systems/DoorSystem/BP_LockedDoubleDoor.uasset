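; Locked double door that rattles when interacted with, with no unlock or opening logic in the Blueprint.
; A Box overlap toggles an Interacting flag without filtering the overlapping actor, and the Interact event acts only while that flag is set.
; Interact starts two timelines, DoorShake and Door2Shake, which drive the yaw of the right and left metal door meshes while keeping their roll and pitch.
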(event OnComponentBeginOverlap(Box)
  (params (OverlappedComponent :type Primitive%20Component%20Object%20Reference) (OtherActor :type Actor%20Object%20Reference) (OtherComp :type Primitive%20Component%20Object%20Reference) (OtherBodyIndex :type Integer) (bFromSweep :type Boolean) (SweepResult :type Hit%20Result%20Structure%20%28by%20ref%29))
  (Variables|Default|SetInteracting? true))

(event OnComponentEndOverlap(Box)
  (params (OverlappedComponent :type Primitive%20Component%20Object%20Reference) (OtherActor :type Actor%20Object%20Reference) (OtherComp :type Primitive%20Component%20Object%20Reference) (OtherBodyIndex :type Integer))
  (Variables|Default|SetInteracting? false))

(event EventBeginPlay)

(event Collision|EventActorBeginOverlap
  (params (OtherActor :type Actor%20Object%20Reference)))

(event EventTick
  (params (DeltaSeconds :type Float%20%28single-precision%29)))

(event EventInteract
  (bind _sm_doormetala_right (Variables|Default|GetSM_DoorMetalA_Right))
  (bind _sm_doormetala_left (Variables|Default|GetSM_DoorMetalA_Left))
  (bind _relativerotation (Variables|/Script/Engine.SceneComponent|GetRelativeRotation _sm_doormetala_right))
  (bind _relativerotation_2 (Variables|/Script/Engine.SceneComponent|GetRelativeRotation _sm_doormetala_left))
  (if (Variables|Default|GetInteracting?)
    (Utilities|FlowControl|Sequence
      (:then_0
        (bind _door (Timeline|DoorShake Play)
          (:Update
            (Transformation|SetRelativeRotation (Variables|Default|GetSM_DoorMetalA_Right) (Math|Rotator|MakeRotator (.roll _relativerotation) (.pitch _relativerotation) _door) false false))))
      (:then_1
        (bind _door2shake (Timeline|Door2Shake Play)
          (:Update
            (Transformation|SetRelativeRotation (Variables|Default|GetSM_DoorMetalA_Left) (Math|Rotator|MakeRotator (.roll _relativerotation_2) (.pitch _relativerotation_2) _door2shake) false false)))))))

(fn ConstructionScript)