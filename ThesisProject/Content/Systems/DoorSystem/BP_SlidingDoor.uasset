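; BP_SlidingDoor is a roller door actor that slides upward when interacted with from inside its trigger box.
; Box overlap begin and end events toggle InArea, without checking which actor overlaps.
; The Interact event checks InArea and that DoorUp is false, then plays the SlideDoorUp timeline to drive the door mesh's relative Z.
; DoorUp is never set here, and no closing logic exists.
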(event OnComponentBeginOverlap(Box)
  (params (OverlappedComponent :type Primitive%20Component%20Object%20Reference) (OtherActor :type Actor%20Object%20Reference) (OtherComp :type Primitive%20Component%20Object%20Reference) (OtherBodyIndex :type Integer) (bFromSweep :type Boolean) (SweepResult :type Hit%20Result%20Structure%20%28by%20ref%29))
  (Variables|Default|SetInArea true))

(event OnComponentEndOverlap(Box)
  (params (OverlappedComponent :type Primitive%20Component%20Object%20Reference) (OtherActor :type Actor%20Object%20Reference) (OtherComp :type Primitive%20Component%20Object%20Reference) (OtherBodyIndex :type Integer))
  (Variables|Default|SetInArea false))

(event EventBeginPlay)

(event Collision|EventActorBeginOverlap
  (params (OtherActor :type Actor%20Object%20Reference)))

(event EventTick
  (params (DeltaSeconds :type Float%20%28single-precision%29)))

(event EventInteract
  (bind _sm_rollerdoor_staticmeshcomponent0 (Variables|Default|GetSM_RollerDoor_StaticMeshComponent0))
  (bind _relativelocation (Variables|/Script/Engine.SceneComponent|GetRelativeLocation _sm_rollerdoor_staticmeshcomponent0))
  (if (Variables|Default|GetInArea)
    (if (not (Variables|Default|GetDoorUp?))
      (bind _slidedoorup (Timeline|SlideDoorUp Play)
        (:Update
          (Transformation|SetRelativeLocation _sm_rollerdoor_staticmeshcomponent0 (Math|Vector|MakeVector (.x _relativelocation) (.y _relativelocation) _slidedoorup) false false))))))

(fn ConstructionScript)