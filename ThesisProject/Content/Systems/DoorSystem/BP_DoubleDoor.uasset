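; Interactable double door that cycles through closed, partially open and fully open, swinging away from the player based on a facing dot product.
; Interact sets the swing side and starts a one-second window in which Tick eases both leaves' yaw toward the next angle with FInterpTo.
; When the timer ends, DoorStop halts movement, plays that step's sound and advances the state.
; Timeline-driven door shake logic is present but never runs.
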(event OnComponentBeginOverlap(Box)
  (params (OverlappedComponent :type Primitive%20Component%20Object%20Reference) (OtherActor :type Actor%20Object%20Reference) (OtherComp :type Primitive%20Component%20Object%20Reference) (OtherBodyIndex :type Integer) (bFromSweep :type Boolean) (SweepResult :type Hit%20Result%20Structure%20%28by%20ref%29)))

(event OnComponentEndOverlap(Box)
  (params (OverlappedComponent :type Primitive%20Component%20Object%20Reference) (OtherActor :type Actor%20Object%20Reference) (OtherComp :type Primitive%20Component%20Object%20Reference) (OtherBodyIndex :type Integer)))

(event Custom|HandleRotation
  (params (SetRotation :type Float%20%28double-precision%29))
  (Transformation|SetRelativeRotation (Variables|Default|GetSM_DoorMetalA_Right) (Math|Rotator|MakeRotator 0.0 0.0 (Math|Interpolation|FInterpTo (.Yaw (Math|Rotator|BreakRotator (Variables|/Script/Engine.SceneComponent|GetRelativeRotation (Variables|Default|GetSM_DoorMetalA_Right)))) SetRotation (Utilities|Time|GetWorldDeltaSeconds) (Variables|Default|GetInterpSpeed))) false false))

(event Custom|HandleDoor
  (switch Utilities|FlowControl|Switch|SwitchonE_DoorStates (Variables|Default|GetDoorStates)
    (:NewEnumerator0
      (CallFunction|HandleRotation (* 15.0 (Variables|Default|GetDoorOpenSide)))
      (CallFunction|HandleRotationLeft (* -15.0 (Variables|Default|GetDoorOpenSide))))
    (:NewEnumerator1
      (CallFunction|HandleRotation (* (Variables|Default|GetDoorOpenAngle) (Variables|Default|GetDoorOpenSide)))
      (CallFunction|HandleRotationLeft (* (Variables|Default|GetDoorOpenAngleLeft) (Variables|Default|GetDoorOpenSide))))
    (:NewEnumerator2
      (CallFunction|HandleRotation 0.0)
      (CallFunction|HandleRotationLeft 0.0))))

(event Custom|Interacting
  (params (Player :type BP%20Third%20Person%20Character%20Object%20Reference))
  (if (> (Math|Vector|DotProduct (Transformation|GetActorForwardVector Player) (Math|Vector|GetForwardVector (Variables|Default|GetDoorOpeningLocation))) 0.0)
    (Variables|Default|SetDoorOpenSide 1.0)
    (else
      (Variables|Default|SetDoorOpenSide -1.0)))
  (Variables|Default|SetInteracting? true)
  (Utilities|Time|SetTimerbyEvent (delegate Custom|DoorStop) 1.0))

(event Custom|DoorStop
  (bind _dooropeninglocation (Variables|Default|GetDoorOpeningLocation))
  (bind _relativelocation (Variables|/Script/Engine.SceneComponent|GetRelativeLocation _dooropeninglocation))
  (Variables|Default|SetInteracting? false)
  (switch Utilities|FlowControl|Switch|SwitchonE_DoorStates (Variables|Default|GetDoorStates)
    (:NewEnumerator0
      (Audio|PlaySoundatLocation "/Game/SFX/SoundEffects/General/DoorOpenPartially.DoorOpenPartially" _relativelocation "0, 0, 0" 1.0 1.0 0.0 0 0 0 0)
      (Variables|Default|SetDoorStates "NewEnumerator1"))
    (:NewEnumerator1
      (Audio|PlaySoundatLocation "/Game/SFX/SoundEffects/General/DoorOpenFull.DoorOpenFull" _relativelocation "0, 0, 0" 1.0 1.0 0.0 0 0 0 0)
      (Variables|Default|SetDoorStates "NewEnumerator2"))
    (:NewEnumerator2
      (Audio|PlaySoundatLocation "/Game/SFX/SoundEffects/General/DoorClosed.DoorClosed" _relativelocation "0, 0, 0" 1.0 1.0 0.0 0 0 0 0)
      (Variables|Default|SetDoorStates "NewEnumerator0"))))

(event Custom|HandleRotationLeft
  (params (SetRotation :type Float%20%28double-precision%29))
  (Transformation|SetRelativeRotation (Variables|Default|GetSM_DoorMetalA_Left) (Math|Rotator|MakeRotator 0.0 0.0 (Math|Interpolation|FInterpTo (.Yaw (Math|Rotator|BreakRotator (Variables|/Script/Engine.SceneComponent|GetRelativeRotation (Variables|Default|GetSM_DoorMetalA_Left)))) SetRotation (Utilities|Time|GetWorldDeltaSeconds) (Variables|Default|GetInterpSpeed))) false false))

(event Collision|EventActorBeginOverlap
  (params (OtherActor :type Actor%20Object%20Reference)))

(event EventTick
  (params (DeltaSeconds :type Float%20%28single-precision%29))
  (if (Variables|Default|GetInteracting?)
    (CallFunction|HandleDoor)))

(event EventBeginPlay
  (bind _asbp_third_person_character (Utilities|Casting|CastToBP_ThirdPersonCharacter (Game|GetPlayerCharacter 0)))
  (Variables|Default|SetAs%20BP%20Third%20Person%20Character _asbp_third_person_character))

(event EventInteract
  (if (not (Variables|Default|GetInteracting?))
    (CallFunction|Interacting (Variables|Default|GetAs%20BP%20Third%20Person%20Character))))

(fn ConstructionScript)