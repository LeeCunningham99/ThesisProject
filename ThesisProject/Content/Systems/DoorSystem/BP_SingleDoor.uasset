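; Single swinging door that the player cycles through closed, partially open and open states, one step per interaction.
; Interact picks the swing side from the dot product of player and door-marker forward vectors, then starts a one-second window that blocks re-triggering.
; During that window, Tick eases the door mesh's yaw with FInterpTo toward the current state's target.
; When the timer ends, motion stops and the state advances.
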(event Custom|Interacting
  (params (Player :type BP%20Third%20Person%20Character%20Object%20Reference))
  ;[1 1 1] Door Interaction Mechanic
  (if (> (Math|Vector|DotProduct (Transformation|GetActorForwardVector Player) (Math|Vector|GetForwardVector (Variables|Default|GetDoorOpeningLocation))) 0.0)
    (Variables|Default|SetDoorOpenSide 1.0)
    (else
      (Variables|Default|SetDoorOpenSide -1.0)))
  (Variables|Default|SetInteracting? true)
  (Utilities|Time|SetTimerbyEvent (delegate Custom|DoorStop) 1.0))

(event Custom|DoorStop
  ;[1 1 1] Door Interaction Mechanic
  (Variables|Default|SetInteracting? false)
  (switch Utilities|FlowControl|Switch|SwitchonE_DoorStates (Variables|Default|GetDoorStates)
    (:NewEnumerator0
      (Variables|Default|SetDoorStates "NewEnumerator1"))
    (:NewEnumerator1
      (Variables|Default|SetDoorStates "NewEnumerator2"))
    (:NewEnumerator2
      (Variables|Default|SetDoorStates "NewEnumerator0"))))

(event Custom|HandleRotation
  (params (SetRotation :type Float%20%28double-precision%29))
  ;[1 1 1] Handle Rotation Of Door
  (Transformation|SetRelativeRotation (Variables|Default|GetDoorMetalC) (Math|Rotator|MakeRotator 0.0 0.0 (Math|Interpolation|FInterpTo (.Yaw (Math|Rotator|BreakRotator (Variables|/Script/Engine.SceneComponent|GetRelativeRotation (Variables|Default|GetDoorMetalC)))) SetRotation (Utilities|Time|GetWorldDeltaSeconds) (Variables|Default|GetInterpSpeed))) false false))

(event Custom|HandleDoor
  ;[1 1 1] Handle Door (Rotating Door Depending On Door State)
  (switch Utilities|FlowControl|Switch|SwitchonE_DoorStates (Variables|Default|GetDoorStates)
    (:NewEnumerator0
      (CallFunction|HandleRotation (* -15.0 (Variables|Default|GetDoorOpenSide))))
    (:NewEnumerator1
      (CallFunction|HandleRotation (* (Variables|Default|GetDoorOpenAngle) (Variables|Default|GetDoorOpenSide))))
    (:NewEnumerator2
      (CallFunction|HandleRotation 0.0))))

(event EventTick
  (params (DeltaSeconds :type Float%20%28single-precision%29))
  ;[1 1 1] Check For Door Opening
  (if (Variables|Default|GetInteracting?)
    (CallFunction|HandleDoor)))

(event EventInteract
  ;[1 1 1] Activate Door Interaction
  (if (not (Variables|Default|GetInteracting?))
    (CallFunction|Interacting (Variables|Default|GetAs%20BP%20Third%20Person%20Character))))

(event EventBeginPlay
  (bind _asbp_third_person_character (Utilities|Casting|CastToBP_ThirdPersonCharacter (Game|GetPlayerCharacter 0)))
  (Variables|Default|SetAs%20BP%20Third%20Person%20Character _asbp_third_person_character))

(fn ConstructionScript)