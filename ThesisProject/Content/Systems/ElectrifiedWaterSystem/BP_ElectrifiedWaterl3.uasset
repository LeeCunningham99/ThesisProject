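; BP_ElectrifiedWaterl3 is an electrified water hazard that ends the game when the player touches it.
; On BeginPlay it caches the player's BP_ThirdPersonCharacter, and its Collision component's begin-overlap event checks for that character.
; On a match it plays a hurt sound, adds the W_GameOverElectricityLEVEL3 widget to the viewport, shows the mouse cursor and pauses the game.
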(event OnComponentBeginOverlap(Collision)
  (params (OverlappedComponent :type Primitive%20Component%20Object%20Reference) (OtherActor :type Actor%20Object%20Reference) (OtherComp :type Primitive%20Component%20Object%20Reference) (OtherBodyIndex :type Integer) (bFromSweep :type Boolean) (SweepResult :type Hit%20Result%20Structure%20%28by%20ref%29))
  (if (== OtherActor (Variables|Default|GetAs%20BP%20Third%20Person%20Character))
    (Audio|PlaySound2D "/Game/SFX/SoundEffects/Player/PlayerHurt.PlayerHurt" 1.0 1.0 0.0 0 0)
    (bind _returnvalue (UserInterface|CreateWidget "/Game/Menus/W_GameOverElectricityLEVEL3.W_GameOverElectricityLEVEL3_C"))
    (bind _output_get (Variables|Default|SetGameOverElectricla _returnvalue))
    (UserInterface|Viewport|AddtoViewport _output_get 0)
    (Variables|/Script/Engine.PlayerController|SetbShowMouseCursor (Game|GetPlayerController 0) true)
    (Game|SetGamePaused true)))

(event EventBeginPlay
  (bind _asbp_third_person_character (Utilities|Casting|CastToBP_ThirdPersonCharacter (Game|GetPlayerCharacter 0)))
  (Variables|Default|SetAs%20BP%20Third%20Person%20Character _asbp_third_person_character))

(event Collision|EventActorBeginOverlap
  (params (OtherActor :type Actor%20Object%20Reference)))

(event EventTick
  (params (DeltaSeconds :type Float%20%28single-precision%29)))

(fn ConstructionScript)