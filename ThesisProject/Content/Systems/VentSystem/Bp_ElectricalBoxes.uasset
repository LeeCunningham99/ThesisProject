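; Easter-egg puzzle actor with eleven electrical boxes that the player switches between red and green materials.
; Overlap volumes flag which box the player stands at, and Interact plays a click and flips that box's material and boolean through a FlipFlop.
; BeginPlay sets boxes 7–11 red, so their FlipFlops run in reverse order to boxes 1–6.
; Tick polls all booleans; when all are true, EasterEggActive roars and destroys an AIGuardSLOW once.
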(event OnComponentBeginOverlap(Collision1)
  (params (OverlappedComponent :type Primitive%20Component%20Object%20Reference) (OtherActor :type Actor%20Object%20Reference) (OtherComp :type Primitive%20Component%20Object%20Reference) (OtherBodyIndex :type Integer) (bFromSweep :type Boolean) (SweepResult :type Hit%20Result%20Structure%20%28by%20ref%29))
  (if (== OtherActor (Variables|Default|GetAs%20BP%20Third%20Person%20Character))
    (Variables|Collision|SetInCollision1 true)))

(event OnComponentEndOverlap(Collision1)
  (params (OverlappedComponent :type Primitive%20Component%20Object%20Reference) (OtherActor :type Actor%20Object%20Reference) (OtherComp :type Primitive%20Component%20Object%20Reference) (OtherBodyIndex :type Integer))
  (if (== OtherActor (Variables|Default|GetAs%20BP%20Third%20Person%20Character))
    (Variables|Collision|SetInCollision1 false)))

(event OnComponentBeginOverlap(Collision6)
  (params (OverlappedComponent :type Primitive%20Component%20Object%20Reference) (OtherActor :type Actor%20Object%20Reference) (OtherComp :type Primitive%20Component%20Object%20Reference) (OtherBodyIndex :type Integer) (bFromSweep :type Boolean) (SweepResult :type Hit%20Result%20Structure%20%28by%20ref%29))
  (if (== OtherActor (Variables|Default|GetAs%20BP%20Third%20Person%20Character))
    (Variables|Collision|SetInCollision6 true)))

(event OnComponentEndOverlap(Collision6)
  (params (OverlappedComponent :type Primitive%20Component%20Object%20Reference) (OtherActor :type Actor%20Object%20Reference) (OtherComp :type Primitive%20Component%20Object%20Reference) (OtherBodyIndex :type Integer))
  (if (== OtherActor (Variables|Default|GetAs%20BP%20Third%20Person%20Character))
    (Variables|Collision|SetInCollision6 false)))

(event OnComponentBeginOverlap(Collision7)
  (params (OverlappedComponent :type Primitive%20Component%20Object%20Reference) (OtherActor :type Actor%20Object%20Reference) (OtherComp :type Primitive%20Component%20Object%20Reference) (OtherBodyIndex :type Integer) (bFromSweep :type Boolean) (SweepResult :type Hit%20Result%20Structure%20%28by%20ref%29))
  (if (== OtherActor (Variables|Default|GetAs%20BP%20Third%20Person%20Character))
    (Variables|Collision|SetInCollision7 true)))

(event OnComponentEndOverlap(Collision7)
  (params (OverlappedComponent :type Primitive%20Component%20Object%20Reference) (OtherActor :type Actor%20Object%20Reference) (OtherComp :type Primitive%20Component%20Object%20Reference) (OtherBodyIndex :type Integer))
  (if (== OtherActor (Variables|Default|GetAs%20BP%20Third%20Person%20Character))
    (Variables|Collision|SetInCollision7 false)))

(event OnComponentBeginOverlap(Collision8)
  (params (OverlappedComponent :type Primitive%20Component%20Object%20Reference) (OtherActor :type Actor%20Object%20Reference) (OtherComp :type Primitive%20Component%20Object%20Reference) (OtherBodyIndex :type Integer) (bFromSweep :type Boolean) (SweepResult :type Hit%20Result%20Structure%20%28by%20ref%29))
  (if (== OtherActor (Variables|Default|GetAs%20BP%20Third%20Person%20Character))
    (Variables|Collision|SetInCollision8 true)))

(event OnComponentEndOverlap(Collision8)
  (params (OverlappedComponent :type Primitive%20Component%20Object%20Reference) (OtherActor :type Actor%20Object%20Reference) (OtherComp :type Primitive%20Component%20Object%20Reference) (OtherBodyIndex :type Integer))
  (if (== OtherActor (Variables|Default|GetAs%20BP%20Third%20Person%20Character))
    (Variables|Collision|SetInCollision8 false)))

(event OnComponentBeginOverlap(Collision9)
  (params (OverlappedComponent :type Primitive%20Component%20Object%20Reference) (OtherActor :type Actor%20Object%20Reference) (OtherComp :type Primitive%20Component%20Object%20Reference) (OtherBodyIndex :type Integer) (bFromSweep :type Boolean) (SweepResult :type Hit%20Result%20Structure%20%28by%20ref%29))
  (if (== OtherActor (Variables|Default|GetAs%20BP%20Third%20Person%20Character))
    (Variables|Collision|SetInCollision9 true)))

(event OnComponentEndOverlap(Collision9)
  (params (OverlappedComponent :type Primitive%20Component%20Object%20Reference) (OtherActor :type Actor%20Object%20Reference) (OtherComp :type Primitive%20Component%20Object%20Reference) (OtherBodyIndex :type Integer))
  (if (== OtherActor (Variables|Default|GetAs%20BP%20Third%20Person%20Character))
    (Variables|Collision|SetInCollision9 false)))

(event OnComponentBeginOverlap(Collision10)
  (params (OverlappedComponent :type Primitive%20Component%20Object%20Reference) (OtherActor :type Actor%20Object%20Reference) (OtherComp :type Primitive%20Component%20Object%20Reference) (OtherBodyIndex :type Integer) (bFromSweep :type Boolean) (SweepResult :type Hit%20Result%20Structure%20%28by%20ref%29))
  (if (== OtherActor (Variables|Default|GetAs%20BP%20Third%20Person%20Character))
    (Variables|Collision|SetInCollision10 true)))

(event OnComponentEndOverlap(Collision10)
  (params (OverlappedComponent :type Primitive%20Component%20Object%20Reference) (OtherActor :type Actor%20Object%20Reference) (OtherComp :type Primitive%20Component%20Object%20Reference) (OtherBodyIndex :type Integer))
  (if (== OtherActor (Variables|Default|GetAs%20BP%20Third%20Person%20Character))
    (Variables|Collision|SetInCollision10 false)))

(event OnComponentBeginOverlap(Collision2)
  (params (OverlappedComponent :type Primitive%20Component%20Object%20Reference) (OtherActor :type Actor%20Object%20Reference) (OtherComp :type Primitive%20Component%20Object%20Reference) (OtherBodyIndex :type Integer) (bFromSweep :type Boolean) (SweepResult :type Hit%20Result%20Structure%20%28by%20ref%29))
  (if (== OtherActor (Variables|Default|GetAs%20BP%20Third%20Person%20Character))
    (Variables|Collision|SetInCollision2 true)))

(event OnComponentBeginOverlap(Collision11)
  (params (OverlappedComponent :type Primitive%20Component%20Object%20Reference) (OtherActor :type Actor%20Object%20Reference) (OtherComp :type Primitive%20Component%20Object%20Reference) (OtherBodyIndex :type Integer) (bFromSweep :type Boolean) (SweepResult :type Hit%20Result%20Structure%20%28by%20ref%29))
  (if (== OtherActor (Variables|Default|GetAs%20BP%20Third%20Person%20Character))
    (Variables|Collision|SetInCollision11 true)))

(event OnComponentEndOverlap(Collision11)
  (params (OverlappedComponent :type Primitive%20Component%20Object%20Reference) (OtherActor :type Actor%20Object%20Reference) (OtherComp :type Primitive%20Component%20Object%20Reference) (OtherBodyIndex :type Integer))
  (if (== OtherActor (Variables|Default|GetAs%20BP%20Third%20Person%20Character))
    (Variables|Collision|SetInCollision11 false)))

(event OnComponentEndOverlap(Collision2)
  (params (OverlappedComponent :type Primitive%20Component%20Object%20Reference) (OtherActor :type Actor%20Object%20Reference) (OtherComp :type Primitive%20Component%20Object%20Reference) (OtherBodyIndex :type Integer))
  (if (== OtherActor (Variables|Default|GetAs%20BP%20Third%20Person%20Character))
    (Variables|Collision|SetInCollision2 false)))

(event OnComponentBeginOverlap(Collision3)
  (params (OverlappedComponent :type Primitive%20Component%20Object%20Reference) (OtherActor :type Actor%20Object%20Reference) (OtherComp :type Primitive%20Component%20Object%20Reference) (OtherBodyIndex :type Integer) (bFromSweep :type Boolean) (SweepResult :type Hit%20Result%20Structure%20%28by%20ref%29))
  (if (== OtherActor (Variables|Default|GetAs%20BP%20Third%20Person%20Character))
    (Variables|Collision|SetInCollision3 true)))

(event OnComponentEndOverlap(Collision3)
  (params (OverlappedComponent :type Primitive%20Component%20Object%20Reference) (OtherActor :type Actor%20Object%20Reference) (OtherComp :type Primitive%20Component%20Object%20Reference) (OtherBodyIndex :type Integer))
  (if (== OtherActor (Variables|Default|GetAs%20BP%20Third%20Person%20Character))
    (Variables|Collision|SetInCollision3 false)))

(event OnComponentBeginOverlap(Collision4)
  (params (OverlappedComponent :type Primitive%20Component%20Object%20Reference) (OtherActor :type Actor%20Object%20Reference) (OtherComp :type Primitive%20Component%20Object%20Reference) (OtherBodyIndex :type Integer) (bFromSweep :type Boolean) (SweepResult :type Hit%20Result%20Structure%20%28by%20ref%29))
  (if (== OtherActor (Variables|Default|GetAs%20BP%20Third%20Person%20Character))
    (Variables|Collision|SetInCollision4 true)))

(event OnComponentEndOverlap(Collision4)
  (params (OverlappedComponent :type Primitive%20Component%20Object%20Reference) (OtherActor :type Actor%20Object%20Reference) (OtherComp :type Primitive%20Component%20Object%20Reference) (OtherBodyIndex :type Integer))
  (if (== OtherActor (Variables|Default|GetAs%20BP%20Third%20Person%20Character))
    (Variables|Collision|SetInCollision4 false)))

(event OnComponentBeginOverlap(Collision5)
  (params (OverlappedComponent :type Primitive%20Component%20Object%20Reference) (OtherActor :type Actor%20Object%20Reference) (OtherComp :type Primitive%20Component%20Object%20Reference) (OtherBodyIndex :type Integer) (bFromSweep :type Boolean) (SweepResult :type Hit%20Result%20Structure%20%28by%20ref%29))
  (if (== OtherActor (Variables|Default|GetAs%20BP%20Third%20Person%20Character))
    (Variables|Collision|SetInCollision5 true)))

(event OnComponentEndOverlap(Collision5)
  (params (OverlappedComponent :type Primitive%20Component%20Object%20Reference) (OtherActor :type Actor%20Object%20Reference) (OtherComp :type Primitive%20Component%20Object%20Reference) (OtherBodyIndex :type Integer))
  (if (== OtherActor (Variables|Default|GetAs%20BP%20Third%20Person%20Character))
    (Variables|Collision|SetInCollision5 false)))

(event Custom|EasterEggActive
  (if (Variables|Default|GetAllActive)
    (Utilities|FlowControl|DoOnce false
      (:Completed
        (bind _returnvalue (Actor|GetActorOfClass "/Game/Systems/Enemies/AIGuard/AIGuardSLOW.AIGuardSLOW_C"))
        (Audio|PlaySound2D "/Game/SFX/SoundEffects/NPC/AlienRoar.AlienRoar" 1.0 1.0 0.0 0 0)
        (Actor|DestroyActor _returnvalue)))))

(event EventBeginPlay
  (bind _asbp_third_person_character (Utilities|Casting|CastToBP_ThirdPersonCharacter (Game|GetPlayerCharacter 0)))
  (Variables|Default|SetAs%20BP%20Third%20Person%20Character _asbp_third_person_character)
  (Rendering|Material|SetMaterial (Variables|Default|GetElectricalBox_7) 0 "/Game/BrutalistLevelKit/Materials/Props/Furniture/Lights/MI_SpringlesRed.MI_SpringlesRed")
  (Rendering|Material|SetMaterial (Variables|Default|GetElectricalBoxRed_8) 0 "/Game/BrutalistLevelKit/Materials/Props/Furniture/Lights/MI_SpringlesRed.MI_SpringlesRed")
  (Rendering|Material|SetMaterial (Variables|Default|GetElectricalBox_9) 0 "/Game/BrutalistLevelKit/Materials/Props/Furniture/Lights/MI_SpringlesRed.MI_SpringlesRed")
  (Rendering|Material|SetMaterial (Variables|Default|GetElectricalBox_10) 0 "/Game/BrutalistLevelKit/Materials/Props/Furniture/Lights/MI_SpringlesRed.MI_SpringlesRed")
  (Rendering|Material|SetMaterial (Variables|Default|GetElectricalBox_11) 0 "/Game/BrutalistLevelKit/Materials/Props/Furniture/Lights/MI_SpringlesRed.MI_SpringlesRed"))

(event Collision|EventActorBeginOverlap
  (params (OtherActor :type Actor%20Object%20Reference)))

(event EventTick
  (params (DeltaSeconds :type Float%20%28single-precision%29))
  (if (Variables|Boxes|GetBox1)
    (if (Variables|Boxes|GetBox2)
      (if (Variables|Boxes|GetBox3)
        (if (Variables|Boxes|GetBox4)
          (if (Variables|Boxes|GetBox5)
            (if (Variables|Boxes|GetBox6)
              (if (Variables|Boxes|GetBox7)
                (if (Variables|Boxes|GetBox8)
                  (if (Variables|Boxes|GetBox9)
                    (if (Variables|Boxes|GetBox10)
                      (if (Variables|Boxes|GetBox11)
                        (Variables|Default|SetAllActive true)
                        (CallFunction|EasterEggActive)))))))))))))

(event EventInteract
  (bind _electricalbox_1 (Variables|Default|GetElectricalBox_1))
  (bind _electricalbox_2 (Variables|Default|GetElectricalBox_2))
  (bind _electricalbox_3 (Variables|Default|GetElectricalBox_3))
  (bind _electricalbox_4 (Variables|Default|GetElectricalBox_4))
  (bind _electricalbox_5 (Variables|Default|GetElectricalBox_5))
  (bind _electricalbox_6 (Variables|Default|GetElectricalBox_6))
  (bind _electricalbox_7 (Variables|Default|GetElectricalBox_7))
  (bind _electricalboxred_8 (Variables|Default|GetElectricalBoxRed_8))
  (bind _electricalbox_9 (Variables|Default|GetElectricalBox_9))
  (bind _electricalbox_10 (Variables|Default|GetElectricalBox_10))
  (bind _electricalbox_11 (Variables|Default|GetElectricalBox_11))
  (if (Variables|Collision|GetInCollision1)
    (Audio|PlaySound2D "/Game/SFX/SoundEffects/General/FlashlightClick.FlashlightClick" 1.0 1.0 0.0 0 0)
    (Utilities|FlowControl|FlipFlop
      (:A
        (Rendering|Material|SetMaterial _electricalbox_1 0 "/Game/BrutalistLevelKit/Materials/Props/Furniture/Lights/MI_SpringlesRed.MI_SpringlesRed")
        (Variables|Default|SetGreenActive false)
        (Variables|Default|SetRedActive true)
        (Variables|Boxes|SetBox1 false))
      (:B
        (Rendering|Material|SetMaterial _electricalbox_1 0 "/Game/BrutalistLevelKit/Materials/Props/Furniture/Lights/MI_Springles.MI_Springles")
        (Variables|Default|SetGreenActive true)
        (Variables|Default|SetRedActive false)
        (Variables|Boxes|SetBox1 true)))
    (elif (Variables|Collision|GetInCollision2)
      (Audio|PlaySound2D "/Game/SFX/SoundEffects/General/FlashlightClick.FlashlightClick" 1.0 1.0 0.0 0 0)
      (Utilities|FlowControl|FlipFlop
        (:A
          (Rendering|Material|SetMaterial _electricalbox_2 0 "/Game/BrutalistLevelKit/Materials/Props/Furniture/Lights/MI_SpringlesRed.MI_SpringlesRed")
          (Variables|Default|SetGreenActive false)
          (Variables|Default|SetRedActive true)
          (Variables|Boxes|SetBox2 false))
        (:B
          (Rendering|Material|SetMaterial _electricalbox_2 0 "/Game/BrutalistLevelKit/Materials/Props/Furniture/Lights/MI_Springles.MI_Springles")
          (Variables|Default|SetGreenActive true)
          (Variables|Default|SetRedActive false)
          (Variables|Boxes|SetBox2 true)))
      (elif (Variables|Collision|GetInCollision3)
        (Audio|PlaySound2D "/Game/SFX/SoundEffects/General/FlashlightClick.FlashlightClick" 1.0 1.0 0.0 0 0)
        (Utilities|FlowControl|FlipFlop
          (:A
            (Rendering|Material|SetMaterial _electricalbox_3 0 "/Game/BrutalistLevelKit/Materials/Props/Furniture/Lights/MI_SpringlesRed.MI_SpringlesRed")
            (Variables|Default|SetGreenActive false)
            (Variables|Default|SetRedActive true)
            (Variables|Boxes|SetBox3 false))
          (:B
            (Rendering|Material|SetMaterial _electricalbox_3 0 "/Game/BrutalistLevelKit/Materials/Props/Furniture/Lights/MI_Springles.MI_Springles")
            (Variables|Default|SetGreenActive true)
            (Variables|Default|SetRedActive false)
            (Variables|Boxes|SetBox3 true)))
        (elif (Variables|Collision|GetInCollision4)
          (Audio|PlaySound2D "/Game/SFX/SoundEffects/General/FlashlightClick.FlashlightClick" 1.0 1.0 0.0 0 0)
          (Utilities|FlowControl|FlipFlop
            (:A
              (Rendering|Material|SetMaterial _electricalbox_4 0 "/Game/BrutalistLevelKit/Materials/Props/Furniture/Lights/MI_SpringlesRed.MI_SpringlesRed")
              (Variables|Default|SetGreenActive false)
              (Variables|Default|SetRedActive true)
              (Variables|Boxes|SetBox4 false))
            (:B
              (Rendering|Material|SetMaterial _electricalbox_4 0 "/Game/BrutalistLevelKit/Materials/Props/Furniture/Lights/MI_Springles.MI_Springles")
              (Variables|Default|SetGreenActive true)
              (Variables|Default|SetRedActive false)
              (Variables|Boxes|SetBox4 true)))
          (elif (Variables|Collision|GetInCollision5)
            (Audio|PlaySound2D "/Game/SFX/SoundEffects/General/FlashlightClick.FlashlightClick" 1.0 1.0 0.0 0 0)
            (Utilities|FlowControl|FlipFlop
              (:A
                (Rendering|Material|SetMaterial _electricalbox_5 0 "/Game/BrutalistLevelKit/Materials/Props/Furniture/Lights/MI_SpringlesRed.MI_SpringlesRed")
                (Variables|Default|SetGreenActive false)
                (Variables|Default|SetRedActive true)
                (Variables|Boxes|SetBox5 false))
              (:B
                (Rendering|Material|SetMaterial _electricalbox_5 0 "/Game/BrutalistLevelKit/Materials/Props/Furniture/Lights/MI_Springles.MI_Springles")
                (Variables|Default|SetGreenActive true)
                (Variables|Default|SetRedActive false)
                (Variables|Boxes|SetBox5 true)))
            (elif (Variables|Collision|GetInCollision6)
              (Audio|PlaySound2D "/Game/SFX/SoundEffects/General/FlashlightClick.FlashlightClick" 1.0 1.0 0.0 0 0)
              (Utilities|FlowControl|FlipFlop
                (:A
                  (Rendering|Material|SetMaterial _electricalbox_6 0 "/Game/BrutalistLevelKit/Materials/Props/Furniture/Lights/MI_SpringlesRed.MI_SpringlesRed")
                  (Variables|Default|SetGreenActive false)
                  (Variables|Default|SetRedActive true)
                  (Variables|Boxes|SetBox6 false))
                (:B
                  (Rendering|Material|SetMaterial _electricalbox_6 0 "/Game/BrutalistLevelKit/Materials/Props/Furniture/Lights/MI_Springles.MI_Springles")
                  (Variables|Default|SetGreenActive true)
                  (Variables|Default|SetRedActive false)
                  (Variables|Boxes|SetBox6 true)))
              (elif (Variables|Collision|GetInCollision7)
                (Audio|PlaySound2D "/Game/SFX/SoundEffects/General/FlashlightClick.FlashlightClick" 1.0 1.0 0.0 0 0)
                (Utilities|FlowControl|FlipFlop
                  (:A
                    (Rendering|Material|SetMaterial _electricalbox_7 0 "/Game/BrutalistLevelKit/Materials/Props/Furniture/Lights/MI_Springles.MI_Springles")
                    (Variables|Default|SetGreenActive true)
                    (Variables|Default|SetRedActive false)
                    (Variables|Boxes|SetBox7 true))
                  (:B
                    (Rendering|Material|SetMaterial _electricalbox_7 0 "/Game/BrutalistLevelKit/Materials/Props/Furniture/Lights/MI_SpringlesRed.MI_SpringlesRed")
                    (Variables|Default|SetGreenActive false)
                    (Variables|Default|SetRedActive true)
                    (Variables|Boxes|SetBox7 false)))
                (elif (Variables|Collision|GetInCollision8)
                  (Audio|PlaySound2D "/Game/SFX/SoundEffects/General/FlashlightClick.FlashlightClick" 1.0 1.0 0.0 0 0)
                  (Utilities|FlowControl|FlipFlop
                    (:A
                      (Rendering|Material|SetMaterial _electricalboxred_8 0 "/Game/BrutalistLevelKit/Materials/Props/Furniture/Lights/MI_Springles.MI_Springles")
                      (Variables|Default|SetGreenActive true)
                      (Variables|Default|SetRedActive false)
                      (Variables|Boxes|SetBox8 true))
                    (:B
                      (Rendering|Material|SetMaterial _electricalboxred_8 0 "/Game/BrutalistLevelKit/Materials/Props/Furniture/Lights/MI_SpringlesRed.MI_SpringlesRed")
                      (Variables|Default|SetGreenActive false)
                      (Variables|Default|SetRedActive true)
                      (Variables|Boxes|SetBox8 false)))
                  (elif (Variables|Collision|GetInCollision9)
                    (Audio|PlaySound2D "/Game/SFX/SoundEffects/General/FlashlightClick.FlashlightClick" 1.0 1.0 0.0 0 0)
                    (Utilities|FlowControl|FlipFlop
                      (:A
                        (Rendering|Material|SetMaterial _electricalbox_9 0 "/Game/BrutalistLevelKit/Materials/Props/Furniture/Lights/MI_Springles.MI_Springles")
                        (Variables|Default|SetGreenActive true)
                        (Variables|Default|SetRedActive false)
                        (Variables|Boxes|SetBox9 true))
                      (:B
                        (Rendering|Material|SetMaterial _electricalbox_9 0 "/Game/BrutalistLevelKit/Materials/Props/Furniture/Lights/MI_SpringlesRed.MI_SpringlesRed")
                        (Variables|Default|SetGreenActive false)
                        (Variables|Default|SetRedActive true)
                        (Variables|Boxes|SetBox9 false)))
                    (elif (Variables|Collision|GetInCollision10)
                      (Audio|PlaySound2D "/Game/SFX/SoundEffects/General/FlashlightClick.FlashlightClick" 1.0 1.0 0.0 0 0)
                      (Utilities|FlowControl|FlipFlop
                        (:A
                          (Rendering|Material|SetMaterial _electricalbox_10 0 "/Game/BrutalistLevelKit/Materials/Props/Furniture/Lights/MI_Springles.MI_Springles")
                          (Variables|Default|SetGreenActive true)
                          (Variables|Default|SetRedActive false)
                          (Variables|Boxes|SetBox10 true))
                        (:B
                          (Rendering|Material|SetMaterial _electricalbox_10 0 "/Game/BrutalistLevelKit/Materials/Props/Furniture/Lights/MI_SpringlesRed.MI_SpringlesRed")
                          (Variables|Default|SetGreenActive false)
                          (Variables|Default|SetRedActive true)
                          (Variables|Boxes|SetBox10 false)))
                      (elif (Variables|Collision|GetInCollision11)
                        (Audio|PlaySound2D "/Game/SFX/SoundEffects/General/FlashlightClick.FlashlightClick" 1.0 1.0 0.0 0 0)
                        (Utilities|FlowControl|FlipFlop
                          (:A
                            (Rendering|Material|SetMaterial _electricalbox_11 0 "/Game/BrutalistLevelKit/Materials/Props/Furniture/Lights/MI_Springles.MI_Springles")
                            (Variables|Default|SetGreenActive true)
                            (Variables|Default|SetRedActive false)
                            (Variables|Boxes|SetBox11 true))
                          (:B
                            (Rendering|Material|SetMaterial _electricalbox_11 0 "/Game/BrutalistLevelKit/Materials/Props/Furniture/Lights/MI_SpringlesRed.MI_SpringlesRed")
                            (Variables|Default|SetGreenActive false)
                            (Variables|Default|SetRedActive true)
                            (Variables|Boxes|SetBox11 false)))))))))))))))

(fn ConstructionScript)