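; BP_Document6 is an interactable document pickup in the Facility that shows its contents on screen when used.
; On Interact it plays a pickup sound, creates the W_Document6 widget and adds it to the viewport.
; It then switches to game-and-UI input with a visible cursor and pauses the game.
; BeginPlay caches the third-person player character, which nothing else in the graph uses.
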(event EventBeginPlay
  (bind _asbp_third_person_character (Utilities|Casting|CastToBP_ThirdPersonCharacter (Game|GetPlayerCharacter 0)))
  (Variables|Default|SetAs%20BP%20Third%20Person%20Character _asbp_third_person_character))

(event EventInteract
  (bind _returnvalue (Game|GetPlayerController 0))
  (Audio|PlaySound2D "/Game/SFX/SoundEffects/General/PickupSound.PickupSound" 1.0 1.0 0.0 0 0)
  (bind _returnvalue_2 (UserInterface|CreateWidget "/Game/Menus/Documents/W_Document6.W_Document6_C" _returnvalue))
  (bind _output_get (Variables|Default|SetNewVar _returnvalue_2))
  (UserInterface|Viewport|AddtoViewport _output_get 0)
  (Input|SetInputModeGameandUI _returnvalue (Variables|Default|GetNewVar) "DoNotLock" false false)
  (Variables|/Script/Engine.PlayerController|SetbShowMouseCursor _returnvalue true)
  (Game|SetGamePaused true))

(fn ConstructionScript)